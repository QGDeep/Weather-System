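; BP_WeatherSystem runs a repeating rain cycle, with randomized start delay and duration, using a Niagara rain effect attached to the player pawn.
; A rain timeline drives storm clouds on a dynamic volumetric cloud material, height fog, particle amount and DoOnce-gated sound fades.
; A material timeline drives wetness through MPC_Weather, holds at full rain, then reverses after the rain timeline so surfaces dry later, restarting the cycle.
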(event `self.ReceiveBeginPlay`
  (bind _volumetriccloud (`self.VolumetricCloud`))
  (`|ExecutionSequence`
    (:`then_0`
      (bind _returnvalue (`NiagaraFunctionLibrary.SpawnSystemAttached` "/Game/WeatherSystem/NS_Rain.NS_Rain" (`Actor.RootComponent` (`Controller.K2_GetPawn` (`GameplayStatics.GetPlayerController` 0))) "None" (0.0 0.0 400.0) (struct) "KeepRelativeOffset")) ; if building are higher, set z axis location higher than 400
      (set `self.Rain_Particles` _returnvalue)
      (bind _returnvalue_2 (`KismetMaterialLibrary.CreateDynamicMaterialInstance` (`|ConvertAsset` (`VolumetricCloudComponent.Material` _volumetriccloud))))
      (bind _output_get (set `self.Cloud_Material` _returnvalue_2))
      (`VolumetricCloudComponent.SetMaterial` _volumetriccloud _output_get))
    (:`then_1`
      (`self.Init_Rain`))))

(event `Init_Rain`
  (set `self.Rain_Start_Delay` (`KismetMathLibrary.RandomFloatInRange` (`self.Rain_Start_Delay_Min`) (`self.Rain_Start_Delay_Max`)))
  (set `self.Rain_Duration` (`KismetMathLibrary.RandomFloatInRange` (`self.Rain_Duration_Min`) (`self.Rain_Duration_Max`)))
  (`KismetSystemLibrary.K2_SetTimer` null "Begin_Rain" (`self.Rain_Start_Delay`))
  (`KismetSystemLibrary.PrintString` "Init Rain"))

(event `Begin_Rain`
  (`KismetSystemLibrary.PrintString` "Begin Rain")
  (`|ExecutionSequence`
    (:`then_0`
      (`TimelineComponent.SetPlayRate` (`self.Rain_Timeline`) (`self.Transition_Speed`))
      (`TimelineComponent.SetPlayRate` (`self.Material_Timeline`) (`self.Transition_Speed`)))
    (:`then_1`
      (bind (_direction _rain_effects) (`Timeline|Rain_Timeline` :!label _label) ; how fast the rain comes in (Spawns)
        (:`Update`
          (`MaterialInstanceDynamic.SetScalarParameterValue` (`self.Cloud_Material`) "StormClouds" (`KismetMathLibrary.Lerp` 0.0 0.975 _rain_effects))
          (`ExponentialHeightFogComponent.SetFogDensity` (`self.ExponentialHeightFog`) (`KismetMathLibrary.Lerp` 0.02 0.8 _rain_effects))
          (`ExponentialHeightFogComponent.SetFogHeightFalloff` (`self.ExponentialHeightFog`) (`KismetMathLibrary.Lerp` 0.2 1.5 _rain_effects))
          (`NiagaraComponent.SetNiagaraVariableFloat` (`self.Rain_Particles`) "Rain_Amount" (`KismetMathLibrary.MapRangeClamped` _rain_effects (`self.Rain_Min_Alpha`) (`self.Rain_Max_Alpha`) 0.0 1.0))
          (switch `ETimelineDirection` _direction
            (:`Forward`
              (if (>= _rain_effects (`self.Rain_Min_Alpha`))
                (`/Engine/EditorBlueprintResources/StandardMacros.DoOnce` false :!label _label_2
                  (:`Completed`
                    (`self.Rain_Sound`
                      (:`then`
                        _)
                      (:`else`
                        (bind _returnvalue (`GameplayStatics.SpawnSound2D` "/Game/SFX_Essentials_FREE_SAMPLE/SFX_Essentials_06_RAIN/Cues/RAINConc_InsJ_Ambience_Rain_Light_01_LOOP_Cue.RAINConc_InsJ_Ambience_Rain_Light_01_LOOP_Cue" 1.0 1.0 0.0 null))
                        (set `self.Rain_Sound` _returnvalue)))
                    (`AudioComponent.FadeIn` (`self.Rain_Sound`) (/ 2.5 (`self.Transition_Speed`)) 1.0 0.0 "Linear")))))
            (:`Backward`
              (if (<= _rain_effects (`self.Rain_Max_Alpha`))
                (`/Engine/EditorBlueprintResources/StandardMacros.DoOnce` false :!label _label_3
                  (:`Completed`
                    (`AudioComponent.FadeOut` (`self.Rain_Sound`) (/ 2.5 (`self.Transition_Speed`)) 0.0 "Linear")))))))))
    (:`then_2`
      (bind (_direction_2 _material_alpha) (`Timeline|Material_Timeline` :!label _label_4) ; how fast the puddles come in (Spawn)
        (:`Update`
          (`KismetMaterialLibrary.SetScalarParameterValue` "/Game/WeatherSystem/MPC_Weather.MPC_Weather" "Rain_Wetness" _material_alpha))
        (:`Finished`
          (switch `ETimelineDirection` _direction_2
            (:`Forward`
              (`KismetSystemLibrary.PrintString` "Rain Full")
              (`KismetSystemLibrary.Delay` (`self.Rain_Duration`))
              (`self.End_Rain`)
              (`KismetSystemLibrary.PrintString` "Rain End"))
            (:`Backward`
              (`self.Init_Rain`)
              (`KismetSystemLibrary.PrintString` "Rain Finished"))))))
    (:`then_3`
      (`self.Reset_Do_Once_Fade_Out`))))

(event `Reset_Do_Once_Fade_In`
  (goto _label_2 :!via `Reset`))

(event `End_Rain`
  (`|ExecutionSequence`
    (:`then_0`
      (goto _label :!via `Reverse`))
    (:`then_1`
      (`KismetSystemLibrary.Delay` (`self.Material_Wetness_Duration`))
      (goto _label_4 :!via `Reverse`))
    (:`then_2`
      (`self.Reset_Do_Once_Fade_In`))))

(event `Reset_Do_Once_Fade_Out`
  (goto _label_3 :!via `Reset`))

(fn `UserConstructionScript`)